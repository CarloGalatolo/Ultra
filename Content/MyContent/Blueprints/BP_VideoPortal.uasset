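; BP_VideoPortal is an actor that plays a video on its Surface component when PlayVideo is called.
; PlayVideo applies the M_MakingReality material, binds StopVideo to the media player's end-reached event, and opens and plays the source unless already playing.
; StopVideo switches the surface to the placeholder video material.
; An unconnected leftover chain would return BP_InteractableSphere to its start depending on its held and physics state.
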(event `Play Video`
  (bind _media_player (`self.Media Player`))
  (`PrimitiveComponent.SetMaterial` (`self.Surface`) 0 "/Game/MyContent/Media/M_MakingReality.M_MakingReality")
  (add `MediaPlayer.OnEndReached` _media_player (delegate `Stop Video`))
  (if (not (`MediaPlayer.IsPlaying` _media_player))
    (`MediaPlayer.OpenSource` _media_player (`self.Media Source`))
    (`MediaPlayer.Play` _media_player)))

(event `Stop Video`
  (`PrimitiveComponent.SetMaterial` (`self.Surface`) 0 "/Game/UltraSceneExercise/Materials/M_PlaceholderVideo.M_PlaceholderVideo"))

(fn `UserConstructionScript`)