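; BP_Hole3 is a hole Blueprint that reacts when a BP_InteractableSphere overlaps it.
; On overlap it runs the parent's handling, casts the other actor to the sphere class, then activates the Niagara component of NiagaraGrass.
; A delayed call to the sphere's EventReappearAtStart is left unconnected and never runs.
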(event `self.ReceiveBeginPlay`)

(event `self.ReceiveActorBeginOverlap`
  (params (OtherActor :type "Actor Object Reference"))
  (`parent.ReceiveActorBeginOverlap` OtherActor)
  (bind _asbp_interactable_sphere (cast `/Game/MyContent/Blueprints/BP_InteractableSphere` OtherActor))
  (`ActorComponent.Activate` (`NiagaraActor.NiagaraComponent` (`self.Niagara Grass`)) true))

(fn `UserConstructionScript`
  (`parent.UserConstructionScript`))