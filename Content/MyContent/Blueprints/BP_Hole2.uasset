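; BP_Hole2 is a trigger actor that reacts when a BP_InteractableSphere overlaps it.
; On overlap it plays the video on a BP_VideoPortal and reports interaction 0 to BP_UltraGameMode through EventInteractionPerformed.
; The portal reference is found with GetActorOfClass in the construction script, so it binds to whichever portal that search returns.
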(event `self.ReceiveBeginPlay`)

(event `self.ReceiveActorBeginOverlap`
  (params (OtherActor :type "Actor Object Reference"))
  (`parent.ReceiveActorBeginOverlap` OtherActor)
  (cast `/Game/MyContent/Blueprints/BP_InteractableSphere` OtherActor)
  (`/Game/MyContent/Blueprints/BP_VideoPortal.Play Video` (`self.Video Portal Ref`))
  (`/Game/MyContent/Blueprints/BP_UltraGameMode.Event Interaction Performed` (cast `/Game/MyContent/Blueprints/BP_UltraGameMode` (`GameplayStatics.GetGameMode`) :!pure true) 0))

(fn `UserConstructionScript`
  (`parent.UserConstructionScript`)
  (bind _returnvalue (`GameplayStatics.GetActorOfClass` "/Game/MyContent/Blueprints/BP_VideoPortal.BP_VideoPortal_C"))
  (set `self.Video Portal Ref` _returnvalue))